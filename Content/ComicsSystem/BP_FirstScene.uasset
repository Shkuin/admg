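; BP_FirstScene is a comics-system trigger actor that shows a scene widget while an overlap is active.
; On begin overlap it enables its input for player 0, copies its Image value to the BP_ADPaperCharacter's ImageIndex, then creates the widget and adds it to the viewport.
; On end overlap it disables that input and removes the widget.
; Neither event checks which actor caused the overlap.
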(event Collision|EventActorBeginOverlap
  (params (OtherActor :type Actor%20Object%20Reference))
  (Input|EnableInput (Game|GetPlayerController 0))
  (bind _asbp_adpaper_character (Utilities|Casting|CastToBP_ADPaperCharacter (Game|GetPlayerCharacter 0)))
  (Variables|/Game/Player/BP_ADPaperCharacter.BP_ADPaperCharacter_C|SetImageIndex _asbp_adpaper_character (Variables|Default|GetImage))
  (bind _returnvalue (UserInterface|CreateWidget "/Game/ComicsSystem/BP_FirstSceneWidget.BP_FirstSceneWidget_C"))
  (UserInterface|Viewport|AddtoViewport _returnvalue 0))

(event Collision|EventActorEndOverlap
  (params (OtherActor :type Actor%20Object%20Reference))
  (Input|DisableInput (Game|GetPlayerController 0))
  (Widget|RemovefromParent (stale Collision|EventActorBeginOverlap _returnvalue)))

(fn ConstructionScript)