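; Player Paper character Blueprint that lets the player interact with nearby objects.
; An interaction sphere tracks overlapping InteractionInterface implementers, either the actor itself or otherwise its components, in an in-range list.
; The Interact input calls Interaction on the first entry, passing the character, and prints a debug message.
; Hardcoded K and G keys destroy the character and increment an image index.
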(event OnComponentBeginOverlap(InterationSphere)
  (params (OverlappedComponent :type Primitive%20Component%20Object%20Reference) (OtherActor :type Actor%20Object%20Reference) (OtherComp :type Primitive%20Component%20Object%20Reference) (OtherBodyIndex :type Integer) (bFromSweep :type Boolean) (SweepResult :type Hit%20Result%20Structure%20%28by%20ref%29))
  (bind _asinteraction_interface (Utilities|Casting|CastToInteractionInterface OtherActor)
    (:then
      (Utilities|Array|AddUnique (Variables|Default|GetInteractablesInRange) _asinteraction_interface))
    (:CastFailed
      (for _array_element (Class|Actor|GetComponentsbyInterface OtherActor "/Game/InteractionInterface.InteractionInterface_C")
        (Utilities|Array|AddUnique (Variables|Default|GetInteractablesInRange) (.AsInteraction%20Interface (Utilities|Casting|CastToInteractionInterface _array_element)))))))

(event OnComponentEndOverlap(InterationSphere)
  (params (OverlappedComponent :type Primitive%20Component%20Object%20Reference) (OtherActor :type Actor%20Object%20Reference) (OtherComp :type Primitive%20Component%20Object%20Reference) (OtherBodyIndex :type Integer))
  (bind _asinteraction_interface (Utilities|Casting|CastToInteractionInterface OtherActor)
    (:then
      (Utilities|Array|RemoveItem (Variables|Default|GetInteractablesInRange) _asinteraction_interface))
    (:CastFailed
      (for _array_element (Class|Actor|GetComponentsbyInterface OtherActor "/Game/InteractionInterface.InteractionInterface_C")
        (Utilities|Array|RemoveItem (Variables|Default|GetInteractablesInRange) (.AsInteraction%20Interface (Utilities|Casting|CastToInteractionInterface _array_element)))))))

(event EventBeginPlay)

(event Collision|EventActorBeginOverlap
  (params (OtherActor :type Actor%20Object%20Reference)))

(event EventTick
  (params (DeltaSeconds :type Float%20%28single-precision%29)))

(event Input|ActionEvents|InputActionInteract
  (params (Key :type Key%20Structure :default "None"))
  (:Pressed
    (if (> (Utilities|Array|Length (Variables|Default|GetInteractablesInRange)) 0)
      (Default|Interaction (Utilities|Array|Get(acopy) (Variables|Default|GetInteractablesInRange)) self)
      (Development|PrintString "Interacted"))))

(event Input|KeyboardEvents|K
  (params (Key :type Key%20Structure :default "None"))
  (:Pressed
    (Actor|DestroyActor)))

(event Input|KeyboardEvents|G
  (params (Key :type Key%20Structure :default "None"))
  (:Pressed
    (bind _result (Math|Integer|IncrementInt (Variables|Default|GetImageIndex))
      (:%20%20
        (Variables|Default|SetImageIndex _result)))))

(fn ConstructionScript)